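; BP_CheckerLight is a placeable indicator light that shows an on/off state as green or red.
; Activate and Deactivate set the point light color, update IsLightOn and, if SoundEnable is set, play the switch sound at the actor's location.
; BeginPlay calls one of them to apply the initial IsLightOn value, so the sound can also play on startup.
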(event `self.ReceiveBeginPlay`
  (if (`self.bIsLightOn`)
    (`self.Activate`)
    (else
      (`self.Deactivate`))))

(event `G2IActivationInterface.Activate`
  (`LightComponent.SetLightColor` (`self.PointLightComponent`) (struct :`G` 1.0 :`A` 1.0) true)
  (set `self.bIsLightOn` true)
  (if (`self.SoundEnable`) :!label _label
    (`GameplayStatics.PlaySoundAtLocation` (`self.SoundSwitch`) (`self.K2_GetActorLocation`) (struct) (`self.SoundVolume`) 1.0 0.0 null null null null)))

(event `G2IActivationInterface.Deactivate`
  (`LightComponent.SetLightColor` (`self.PointLightComponent`) (struct :`R` 1.0 :`A` 1.0) true)
  (set `self.bIsLightOn` false)
  (goto _label))

(fn `UserConstructionScript`)