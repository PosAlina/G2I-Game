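; Test placeable gear that spins about world X when shot and drives a linked Movable object.
; OnShoot prints a debug vector and restarts a timeline whose curve scales the per-update roll step.
; Spin direction is the sign derived from the impact normal and shot direction flattened to the YZ plane.
; Each update also passes that signed step to Movable through G2IMovingByGearObjectInterface, if implemented.
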(event `G2ITraceableObectInterface.OnShoot`
  (params (HitResult :type "HitResult Structure (by ref)") (Character :type "Actor Object Reference"))
  (bind (_bblockinghit _binitialoverlap _time _distance _location _impactpoint _normal _impactnormal _physmat _hitactor _hitcomponent _hitbonename _bonename _hititem _elementindex _faceindex _tracestart) (`GameplayStatics.BreakHitResult` HitResult))
  (bind _movable (`self.Movable`))
  (bind _returnvalue (`KismetMathLibrary.Cross_VectorVector` (0.0 0.0 1.0) (* _impactnormal (0.0 1.0 1.0))))
  (`KismetSystemLibrary.PrintString` (`KismetStringLibrary.Conv_VectorToString` _returnvalue))
  (bind (_direction _newtrack_0) (`Timeline|RotatorTimeline` :!via `PlayFromStart`)
    (:`Update`
      (if (`KismetSystemLibrary.DoesImplementInterface` _movable "/Script/G2I.G2IMovingByGearObjectInterface")
        (bind _returnvalue_2 (* (`KismetMathLibrary.SignOfFloat` (* (.x _returnvalue) 20.0 (`KismetMathLibrary.Vector_CosineAngle2D` (1.0 0.0 0.0) (`KismetMathLibrary.MakeVector` (.z (* (- _impactpoint _tracestart) (0.0 1.0 1.0))) (.y (* (- _impactpoint _tracestart) (0.0 1.0 1.0))))) _newtrack_0)) 5.0 _newtrack_0))
        (message `G2IMovingByGearObjectInterface.OnPushing` _movable _returnvalue_2))
      (`self.K2_AddActorWorldRotation` (`KismetMathLibrary.MakeRotator` _returnvalue_2)))))

(fn `UserConstructionScript`)