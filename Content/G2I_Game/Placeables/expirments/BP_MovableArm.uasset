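; Movable arm that travels along a referenced spline and picks up and drops actors.
; Pushes adjust a clamped 0–1 position along the spline, while Activate runs a vertical timeline offset that locks pushing until finished.
; Overlapping FDADSDA attaches an actor, hiding its physics-simulating meshes and showing the others.
; Activating while holding detaches it, reverses that visibility swap and re-enables overlaps after a short delay.
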(event `G2IMovingByGearObjectInterface.OnPushing`
  (params (ForceMagnitude :type "Float (single-precision)"))
  (bind _returnvalue (+ (`self.force`) (* (/ ForceMagnitude (`self.MaxForce`)) -1.0)))
  (if (not (`self.Lock`))
    (if (< _returnvalue 0.0)
      (set `self.force` 0.0)
      (elif (> _returnvalue 1.0)
        (set `self.force` 1.0)
        (else
          (set `self.force` _returnvalue))))
    (`self.K2_AddActorWorldOffset` (- (`SplineComponent.GetLocationAtTime` (`self.GetComponentByClass` (`self.SplineActor`) "/Script/Engine.SplineComponent") (`self.force`) "World" false) (`self.K2_GetActorLocation`)))))

(event `self.ReceiveBeginPlay`
  (`self.K2_SetActorLocation` (`SplineComponent.GetLocationAtTime` (`self.GetComponentByClass` (`self.SplineActor`) "/Script/Engine.SplineComponent") 0.0 "World" false)))

(event `G2IActivationInterface.Activate`
  (if (`KismetSystemLibrary.IsValid` (`self.Actor`))
    (`KismetSystemLibrary.PrintString` "Detach")
    (`self.K2_DetachFromActor` (`self.Actor`) "KeepWorld" "KeepWorld" "KeepWorld")
    (for _array_element (`self.K2_GetComponentsByClass` (`self.Actor`) "/Script/Engine.StaticMeshComponent")
      (if (`SceneComponent.IsSimulatingPhysics` _array_element "None")
        (`SceneComponent.SetVisibility` _array_element true true)
        (else
          (`SceneComponent.SetVisibility` _array_element false true)
          (`KismetSystemLibrary.PrintString` (`KismetSystemLibrary.GetDisplayName` _array_element)))))
    (set `self.Actor` null)
    (`KismetSystemLibrary.Delay` 0.5)
    (set `PrimitiveComponent.bGenerateOverlapEvents` true (`self.FDADSDA`))
    (elif (not (`self.Lock`))
      (set `self.Lock` true)
      (set `self.StartLocation` (`self.K2_GetActorLocation`))
      (bind (_direction _newtrack_0) (`Timeline|HeightTimeline` :!via `PlayFromStart`)
        (:`Update`
          (`self.K2_AddActorWorldOffset` (- (+ (`self.StartLocation`) (`KismetMathLibrary.MakeVector` 0.0 0.0 (* _newtrack_0 (`self.DeltaHeight`) -1.0))) (`self.K2_GetActorLocation`))))
        (:`Finished`
          (set `self.Lock` false))))))

(event `self.FDADSDA.OnComponentBeginOverlap`
  (params (OverlappedComponent :type "PrimitiveComponent Object Reference") (OtherActor :type "Actor Object Reference") (OtherComp :type "PrimitiveComponent Object Reference") (OtherBodyIndex :type Integer) (bFromSweep :type Boolean) (SweepResult :type "HitResult Structure (by ref)"))
  (if (not (`KismetSystemLibrary.IsValid` (`self.Actor`)))
    (for _array_element (`self.K2_GetComponentsByClass` OtherActor "/Script/Engine.StaticMeshComponent")
      (if (`SceneComponent.IsSimulatingPhysics` _array_element "None")
        (`SceneComponent.SetVisibility` _array_element false true)
        (else
          (`SceneComponent.SetVisibility` _array_element true true))))
    (bind _output_get (set `self.Actor` OtherActor))
    (`self.K2_AttachToActor` _output_get self "None" "KeepWorld" "KeepWorld" "KeepWorld" false)
    (`KismetSystemLibrary.PrintString` "Attached")
    (set `PrimitiveComponent.bGenerateOverlapEvents` false (`self.FDADSDA`))))

(fn `UserConstructionScript`)