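; Test placeable box that gets pushed horizontally along the direction of a shot when OnShoot fires.
; Each hit restarts a timeline whose curve scales PushSpeed into per-update swept moves of the static mesh.
; On a blocking hit it either reverses at a tenth of the push if Bouncing, or stops and nudges off the surface along its normal.
; Debug lines trace each movement step.
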(event `G2ITraceableObectInterface.OnShoot`
  (params (HitResult :type "HitResult Structure (by ref)") (Character :type "Actor Object Reference"))
  (bind (_bblockinghit _binitialoverlap _time _distance _location _impactpoint _normal _impactnormal _physmat _hitactor _hitcomponent _hitbonename _bonename _hititem _elementindex _faceindex _tracestart) (`GameplayStatics.BreakHitResult` HitResult))
  (bind _staticmesh (`self.StaticMesh`))
  (bind _returnvalue (`SceneComponent.K2_GetComponentLocation` (`self.StaticMesh`)))
  (set `self.multiplier` 1.0)
  (bind (_direction _newtrack_0) (`Timeline|FreakTimeline` :!via `PlayFromStart`)
    (:`Update`
      (bind _returnvalue_2 (+ (* (* (`KismetMathLibrary.Normal` (- _location _tracestart)) (1.0 1.0 0.0)) (`self.PushSpeed`) _newtrack_0 (`self.multiplier`)) _returnvalue))
      (`KismetSystemLibrary.DrawDebugLine` _returnvalue _returnvalue_2 (struct) 3.0)
      (bind _sweephitresult (`SceneComponent.K2_SetWorldLocation` (`self.StaticMesh`) _returnvalue_2 true false))
      (bind (_bblockinghit_2 _binitialoverlap_2 _time_2 _distance_2 _location_2 _impactpoint_2 _normal_2) (`GameplayStatics.BreakHitResult` _sweephitresult))
      (if _bblockinghit_2
        (if (`self.bBouncing`)
          (set `self.multiplier` (* (`self.multiplier`) -0.1))
          (else
            (set `self.multiplier` 0.0)
            (`SceneComponent.K2_SetWorldLocation` _staticmesh (+ (`SceneComponent.K2_GetComponentLocation` _staticmesh) (* _normal_2 (10.0 10.0 0.0))) true false)))))))

(fn `UserConstructionScript`)