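; Test placeable box that the Engineer character can interact with to pick up and release.
; CanInteract accepts only G2ICharacterEngineer and prints a debug string.
; Interact toggles IsMoving: grabbing attaches the box to the interactor, ignores Pawn collision and removes player 0's IMC_Engineer mapping context, while releasing reverses all three.
; GetSpeedChange exposes a SpeedChange value, and the key hint getter returns nothing.
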(event `self.Interact`
  (params (Interactor :type "Character Object Reference"))
  (if (`self.bIsMoving`)
    (`EnhancedInputSubsystemInterface.AddMappingContext` (pcsubsystem `EnhancedInputLocalPlayerSubsystem` (`GameplayStatics.GetPlayerController` 0)) "/Game/G2I_Game/Core/Input/IMC/IMC_Engineer.IMC_Engineer" 0 (struct))
    (`self.K2_DetachFromActor` "KeepWorld" "KeepWorld" "KeepWorld")
    (`PrimitiveComponent.SetCollisionResponseToChannel` (`self.Cube`) "ECC_Pawn" "ECR_Block")
    (set `self.bIsMoving` false)
    (else
      (`EnhancedInputSubsystemInterface.RemoveMappingContext` (pcsubsystem `EnhancedInputLocalPlayerSubsystem` (`GameplayStatics.GetPlayerController` 0)) "/Game/G2I_Game/Core/Input/IMC/IMC_Engineer.IMC_Engineer" (struct))
      (`self.K2_AttachToActor` Interactor "None" "KeepWorld" "KeepWorld" "KeepWorld")
      (`PrimitiveComponent.SetCollisionResponseToChannel` (`self.Cube`) "ECC_Pawn" "ECR_Ignore")
      (set `self.bIsMoving` true))))

(fn `CanInteract`
  (params (Interactor :type "Character Object Reference"))
  (returns (ReturnValue :type Boolean))
  (`KismetSystemLibrary.PrintString` "Hello")
  (cast `G2ICharacterEngineer` Interactor
    (:`then`
      (return true))
    (:`CastFailed`
      (return false))))

(fn `GetInteractionKeyHintComponent`
  (returns (ReturnValue :type "G2IWorldHintKeyWidgetComponent Object Reference"))
  (return null))

(fn `GetSpeedChange`
  (returns (ReturnValue :type "Float (single-precision)"))
  (return (`self.SpeedChange`)))

(fn `UserConstructionScript`)