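; A placeable moving actor that slides its static mesh by a velocity vector while activated.
; Activate and Deactivate switch actor tick on and off, with IsActive choosing the state at BeginPlay.
; Each tick teleports the mesh by a fixed, frame-rate-dependent local offset without sweep.
; Absolute travel accumulates on axes with a nonzero max offset, and exceeding any limit stops the tick.
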(event `self.ReceiveBeginPlay`
  (if (`self.IsActive`)
    (`self.SetActorTickEnabled` true)
    (else
      (`self.SetActorTickEnabled` false))))

(event `self.ReceiveTick`
  (params (DeltaSeconds :type "Float (single-precision)"))
  (bind (_velocity_vector_x _velocity_vector_y _velocity_vector_z) (`KismetMathLibrary.BreakVector` (`self.Velocity Vector`)))
  (bind _velocity_vector_x_2 (`KismetMathLibrary.BreakVector` (`self.Velocity Vector`)))
  (bind (_velocity_vector_x_3 _velocity_vector_y_2) (`KismetMathLibrary.BreakVector` (`self.Velocity Vector`)))
  (`SceneComponent.K2_AddLocalOffset` (`self.StaticMeshComponent`) (`self.Velocity Vector`) false true)
  (`|ExecutionSequence`
    (:`then_0`
      (if (not (== 0.0 (`self.Max OffsetZ`)))
        (set `self.Local OffsetZ` (+ (`self.Local OffsetZ`) (`KismetMathLibrary.Abs` _velocity_vector_z)))
        (if (< (`self.Max OffsetZ`) (`self.Local OffsetZ`))
          (`self.SetActorTickEnabled` false))))
    (:`then_1`
      (if (not (== 0.0 (`self.Max OffsetY`)))
        (set `self.Local OffsetY` (+ (`self.Local OffsetY`) (`KismetMathLibrary.Abs` _velocity_vector_y_2)))
        (if (< (`self.Max OffsetY`) (`self.Local OffsetY`))
          (`self.SetActorTickEnabled` false))))
    (:`then_2`
      (if (not (== 0.0 (`self.Max OffsetX`)))
        (set `self.Local OffsetX` (+ (`self.Local OffsetX`) (`KismetMathLibrary.Abs` _velocity_vector_x_2)))
        (if (< (`self.Max OffsetX`) (`self.Local OffsetX`))
          (`self.SetActorTickEnabled` false))))))

(event `G2IActivationInterface.Deactivate`
  (`self.SetActorTickEnabled` false))

(event `G2IActivationInterface.Activate`
  (`self.SetActorTickEnabled` true))

(fn `UserConstructionScript`)