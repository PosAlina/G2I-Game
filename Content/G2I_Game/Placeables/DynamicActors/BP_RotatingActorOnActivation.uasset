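; Placeable actor that spins by a fixed local rotation each tick, either from BeginPlay when IsActive or once Activate fires.
; Unless limits are ignored, it accumulates absolute rotation per axis and disables tick after exceeding any nonzero maximum.
; Deactivate either disables tick or restores the starting rotation, which leaves tick state and accumulated totals unchanged.
; Rotation is not scaled by delta time, so speed depends on frame rate.
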(event `self.ReceiveBeginPlay`
  (set `self.StartVector` (`self.K2_GetActorRotation`))
  (if (`self.is_active`)
    (`self.SetActorTickEnabled` true)
    (else
      (`self.SetActorTickEnabled` false))))

(event `self.ReceiveTick`
  (params (DeltaSeconds :type "Float (single-precision)"))
  (bind (_rotation_vector_roll _rotation_vector_pitch) (`KismetMathLibrary.BreakRotator` (`self.Rotation vector`)))
  (bind (_rotation_vector_roll_2 _rotation_vector_pitch_2 _rotation_vector_yaw) (`KismetMathLibrary.BreakRotator` (`self.Rotation vector`)))
  (bind _rotation_vector_roll_3 (`KismetMathLibrary.BreakRotator` (`self.Rotation vector`)))
  (`self.K2_AddActorLocalRotation` (`self.Rotation vector`))
  (if (not (`self.IgnoreLimits`))
    (`|ExecutionSequence`
      (:`then_0`
        (if (not (== 0.0 (`self.Max Rotation X`)))
          (set `self.Local Rotation X` (+ (`KismetMathLibrary.Abs` _rotation_vector_roll_3) (`self.Local Rotation X`)))
          (if (< (`self.Max Rotation X`) (`self.Local Rotation X`))
            (`self.SetActorTickEnabled` false))))
      (:`then_1`
        (if (not (== 0.0 (`self.Max Rotation Y`)))
          (set `self.Local Rotation Y` (+ (`KismetMathLibrary.Abs` _rotation_vector_pitch) (`self.Local Rotation Y`)))
          (if (< (`self.Max Rotation Y`) (`self.Local Rotation Y`))
            (`self.SetActorTickEnabled` false))))
      (:`then_2`
        (if (not (== 0.0 (`self.Max Rotation Z`)))
          (set `self.Local Rotation Z` (+ (`KismetMathLibrary.Abs` _rotation_vector_yaw) (`self.Local Rotation Z`)))
          (if (< (`self.Max Rotation Z`) (`self.Local Rotation Z`))
            (`self.SetActorTickEnabled` false)))))))

(event `G2IActivationInterface.Deactivate`
  (if (`self.ResetOnDeactivation`)
    (`self.K2_SetActorRotation` (`self.StartVector`) true)
    (else
      (`self.SetActorTickEnabled` false))))

(event `G2IActivationInterface.Activate`
  (`self.SetActorTickEnabled` true))

(fn `UserConstructionScript`)