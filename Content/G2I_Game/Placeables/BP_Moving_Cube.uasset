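; BP_Moving_Cube is a placeable static-mesh mover that travels a limited vertical distance while active.
; IsActive sets whether Tick runs at BeginPlay, and the Activate and Deactivate events switch Tick on or off.
; Each Tick teleports the mesh by VelocityVector in local space without sweep or delta-time scaling.
; Absolute Z movement accumulates in LocalOffsetZ, and Tick stops once it exceeds MaxOffsetZ, with no reset or reversal.
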(event `self.ReceiveBeginPlay`
  (if (`self.IsActive`)
    (`self.SetActorTickEnabled` true)
    (else
      (`self.SetActorTickEnabled` false))))

(event `self.ReceiveTick`
  (params (DeltaSeconds :type "Float (single-precision)"))
  (bind (_velocity_vector_x _velocity_vector_y _velocity_vector_z) (`KismetMathLibrary.BreakVector` (`self.Velocity Vector`)))
  (`SceneComponent.K2_AddLocalOffset` (`self.StaticMeshComponent`) (`self.Velocity Vector`) false true)
  (set `self.Local OffsetZ` (+ (`self.Local OffsetZ`) (`KismetMathLibrary.Abs` _velocity_vector_z)))
  (if (< (`self.Max OffsetZ`) (`self.Local OffsetZ`))
    (`self.SetActorTickEnabled` false)))

(event `G2IActivationInterface.Deactivate`
  (`self.SetActorTickEnabled` false))

(event `G2IActivationInterface.Activate`
  (`self.SetActorTickEnabled` true))

(fn `UserConstructionScript`)