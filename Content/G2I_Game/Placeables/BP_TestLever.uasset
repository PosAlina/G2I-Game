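; BP_TestLever is a test lever placeable that only an engineer character can interact with.
; CanInteract prints a debug message and allows interaction only when the interactor casts to G2ICharacterEngineer.
; On Interact, it loops over ActorToActivate and calls Activate on each actor and each of its components implementing G2IActivationInterface.
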(event `G2IInteractiveObjectInterface.Interact`
  (params (Interactor :type "Character Object Reference"))
  (for _array_element (`self.ActorToActivate`)
    (bind _asg2iactivation_interface (cast `G2IActivationInterface` _array_element)
      (:`then`
        (`G2IActivationInterface.Activate` _asg2iactivation_interface))
      (:`CastFailed`
        _))
    (for _array_element_2 (`self.GetComponentsByInterface` _array_element "/Script/G2I.G2IActivationInterface")
      (bind _asg2iactivation_interface_2 (cast `G2IActivationInterface` _array_element_2))
      (`G2IActivationInterface.Activate` _asg2iactivation_interface_2))))

(fn `CanInteract`
  (params (Interactor :type "Character Object Reference"))
  (returns (ReturnValue :type Boolean))
  (`KismetSystemLibrary.PrintString` "Hello")
  (cast `G2ICharacterEngineer` Interactor
    (:`then`
      (return true))
    (:`CastFailed`
      (return false))))

(fn `UserConstructionScript`)