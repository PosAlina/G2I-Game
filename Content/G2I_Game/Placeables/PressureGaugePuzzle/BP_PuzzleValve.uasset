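; BP_PuzzleValve is an interactable valve in the pressure gauge puzzle that changes an angle through its linked Puzzle.
; Interacting while it is not rotating toggles the valve, then sends ChangeAngleMessage with its Y value and open state to the target cached at BeginPlay.
; An Answer event disables interaction when the answer is right and allows it otherwise, through the CanOpen flag read by CanInteract.
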(event `self.ReceiveBeginPlay`
  (bind _result (`BlueprintSetLibrary.Set_ToArray` (`self.Puzzle`)))
  (set `self.Target` _result))

(event `G2IInteractiveObjectInterface.Interact`
  (params (Interactor :type "Character Object Reference"))
  (if (not (`self.bIsRotating`))
    (`self.ToggleValve`)
    (message `G2IRotationComponentsInterface.ChangeAngle` (`self.Target`) (`self.Y`) (`self.bIsValveOpen`))))

(event `G2IRotationComponentsInterface.Answer`
  (params (bIsRight :type Boolean))
  (set `self.bCanOpen` (not bIsRight)))

(fn `CanInteract`
  (params (Interactor :type "Character Object Reference"))
  (returns (ReturnValue :type Boolean))
  (return (`self.bCanOpen`)))

(fn `GetInteractionKeyHintComponent`
  (returns (ReturnValue :type "G2IWorldHintKeyWidgetComponent Object Reference"))
  (return null))

(fn `UserConstructionScript`)