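; Pressure gauge puzzle actor that turns three arrows and reports whether they sit at their target angles.
; BeginPlay registers the arrow components and copies PuzzleActors into the Actors array.
; ChangeAngle passes angle deltas and an on/off flag to ArrowsAngle, then checks target angles with a small tolerance and sends the result to Actors through AnswerMessage.
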(event `self.ReceiveBeginPlay`
  (`self.InitializeArrowsComponent` (`|MakeArray` (`self.Arrow`) (`self.Arrow1`) (`self.Arrow2`)))
  (bind _result (`BlueprintSetLibrary.Set_ToArray` (`self.PuzzleActors`)))
  (set `self.Actors` _result))

(event `G2IRotationComponentsInterface.ChangeAngle`
  (params (Y :type "Array of Float (single-precision) (by ref)") (bIsOn :type Boolean))
  (`self.ArrowsAngle` bIsOn Y)
  (message `G2IRotationComponentsInterface.Answer` (`self.Actors`) (`self.CheckTargetAngles` 1.0)))

(fn `UserConstructionScript`)