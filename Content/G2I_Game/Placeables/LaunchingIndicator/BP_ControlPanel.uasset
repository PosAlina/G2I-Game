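; BP_ControlPanel is a placeable control panel from the launching indicator set, carrying a pressure gauge, pipes and eight slider lamps.
; On BeginPlay it passes all of these components as one ordered array to InitializeLamps, then calls the parent BeginPlay.
; The Blueprint only wires up the components, with no indicator behavior of its own and an empty construction script.
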(event `self.ReceiveBeginPlay`
  (`self.InitializeLamps` (`|MakeArray` (`self.PressureGauge`) (`self.Pipes`) (`self.G2ISliderLamp2`) (`self.G2ISliderLamp1`) (`self.G2ISliderLamp`) (`self.G2ISliderLamp7`) (`self.G2ISliderLamp6`) (`self.G2ISliderLamp3`) (`self.G2ISliderLamp5`) (`self.G2ISliderLamp4`)))
  (`parent.ReceiveBeginPlay`))

(fn `UserConstructionScript`)